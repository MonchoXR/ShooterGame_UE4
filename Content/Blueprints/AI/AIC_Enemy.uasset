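; AI controller for enemies, holding logic to run BT_Enemy and feed its blackboard, though none of it is wired to run.
; One disconnected chain starts the tree and copies patrol path settings from the controlled RP_Enemy.
; The other reads perception of player characters, mapping stimuli by array index: sight sets visibility, damage sets investigation and target location.
; BeginPlay and the construction script are empty.
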(event `self.ReceiveBeginPlay`)

(fn `UserConstructionScript`)