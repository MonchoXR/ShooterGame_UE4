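; Player character Blueprint with selectable first or third person view and feedback for an ultimate ability.
; The construction script sets camera and spring arm auto-activation from a view flag, and BeginPlay adds the sight widget and caches the post-process settings.
; Ultimate start and stop events swap between ultimate and cached post-process looks.
; XP gain prints color-coded debug progress, while the duration update is empty and other debug prints are disconnected.
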(event `self.BP_GainUltimateXP`
  (params (XPGained :type "Float (single-precision)"))
  (`KismetSystemLibrary.PrintString` (`KismetStringLibrary.Concat_StrStr` "XP Gained:" (`KismetStringLibrary.Conv_DoubleToString` XPGained) " ||  UltimateXP. " (`KismetStringLibrary.Conv_DoubleToString` (`self.CurrentUltimateXP`)) "/" (`KismetStringLibrary.Conv_DoubleToString` (`self.MaxUltimateXP`))) true true (select `bool` (`self.bCanUseUltimate`) :`false` (struct :`R` 0.35 :`G` 0.875632 :`B` 1.0 :`A` 1.0) :`true` (struct :`R` 0.006967 :`G` 0.995833 :`A` 1.0) :!type "LinearColor Structure") 5.0))

(event `self.ReceiveBeginPlay`
  (`|ExecutionSequence`
    (:`then_0`
      (bind _returnvalue (`|CreateWidget` "/Game/Widgets/BP_Sight.BP_Sight_C"))
      (`UserWidget.AddToViewport` _returnvalue 0))
    (:`then_1`
      (set `self.NormalPostProcess` (`PostProcessComponent.Settings` (`self.PostProcess`))))))

(event `self.BP_StartUltimate`
  (set `PostProcessComponent.Settings` (`self.UltimatePostProcess`) (`self.PostProcess`)))

(event `self.BP_StopUltimate`
  (set `PostProcessComponent.Settings` (`self.NormalPostProcess`) (`self.PostProcess`)))

(event `self.BP_UpdateUltimateDuration`
  (params (Value :type "Float (single-precision)")))

(fn `UserConstructionScript`
  (`ActorComponent.SetAutoActivate` (`self.FPSCameraComponent`) (`self.bUseFirsPersonView`))
  (`ActorComponent.SetAutoActivate` (`self.TPSCameraComponent`) (not (`self.bUseFirsPersonView`)))
  (`ActorComponent.SetAutoActivate` (`self.SpringArmComponent`) (not (`self.bUseFirsPersonView`))))